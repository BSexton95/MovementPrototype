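; Player character Blueprint that handles walking, mouse look and sprinting from input bindings.
; Movement axes push along the Camera component's forward and right vectors, look axes drive controller pitch and yaw, and Sprint switches max walk speed while held.
; A world-space idle camera anim plays on BeginPlay, and the forward/back axis event also starts an idle camera shake and reapplies max walk speed on every call.
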(event EventBeginPlay
  (Class|PlayerCameraManager|PlayCameraAnim (Game|GetPlayerCameraManager 0) "/Game/Animations/Camera_IdleAnim.Camera_IdleAnim" 1.0 1.0 0.0 0.0 false false 0.0 "World" "0, 0, 0"))

(event Collision|EventActorBeginOverlap
  (params (OtherActor :type Actor%20Object%20Reference)))

(event EventTick
  (params (DeltaSeconds :type Float%20%28single-precision%29)))

(event Input|ActionEvents|InputActionSprint
  (params (Key :type Key%20Structure :default "None"))
  (bind _charactermovement (Variables|Character|GetCharacterMovement))
  ;[1 1 1] Sprint
  (:Pressed
    (Variables|/Script/Engine.CharacterMovementComponent|SetMaxWalkSpeed _charactermovement 1e+03))
  (:Released
    (Variables|/Script/Engine.CharacterMovementComponent|SetMaxWalkSpeed _charactermovement 3e+02)))

(event Input|AxisEvents|InputAxisMoveForwardBackward
  (params (AxisValue :type Float%20%28single-precision%29))
  ;[1 1 1] Player Movement Input
  (Class|MatineeCameraShake|StartMatineeCameraShake (Game|GetPlayerCameraManager 0) "/Game/Blueprints/Camera_Idle.Camera_Idle_C" 1.0 "World" "0, 0, 0")
  (Variables|/Script/Engine.CharacterMovementComponent|SetMaxWalkSpeed (Variables|/Script/Engine.Character|GetCharacterMovement (Game|GetPlayerCharacter 0)) (Class|MovementComponent|GetMaxSpeed (Variables|Character|GetCharacterMovement)))
  (Pawn|Input|AddMovementInput (Math|Vector|GetForwardVector (Variables|Character|GetCamera)) AxisValue false))

(event Input|AxisEvents|InputAxisMoveLeftRight
  (params (AxisValue :type Float%20%28single-precision%29))
  ;[1 1 1] Player Movement Input
  (Pawn|Input|AddMovementInput (Math|Vector|GetRightVector (Variables|Character|GetCamera)) AxisValue false))

(event Input|AxisEvents|InputAxisLookUpDown
  (params (AxisValue :type Float%20%28single-precision%29))
  ;[1 1 1] Mouse View Input
  (Pawn|Input|AddControllerPitchInput AxisValue))

(event Input|AxisEvents|InputAxisLookLeftRight
  (params (AxisValue :type Float%20%28single-precision%29))
  ;[1 1 1] Mouse View Input
  (Pawn|Input|AddControllerYawInput AxisValue))

(fn ConstructionScript)